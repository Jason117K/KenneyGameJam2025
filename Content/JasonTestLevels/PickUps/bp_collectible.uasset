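; Collectible pickup actor that adds to the player's collectable count when touched.
; A Box overlap event checks that the overlapping actor is the first player's pawn, then casts that player's state to ball_player_state.
; It increments CollectableCount there, prints the new total to screen and destroys itself.
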(event `self.Box.OnComponentBeginOverlap`
  (params (OverlappedComponent :type "PrimitiveComponent Object Reference") (OtherActor :type "Actor Object Reference") (OtherComp :type "PrimitiveComponent Object Reference") (OtherBodyIndex :type Integer) (bFromSweep :type Boolean) (SweepResult :type "HitResult Structure (by ref)"))
  (if (== OtherActor (`GameplayStatics.GetPlayerPawn` 0))
    (bind _asball_player_state (cast `/Game/JasonTestLevels/ball_player_state` (`GameplayStatics.GetPlayerState` 0)))
    (bind _output_get (set `/Game/JasonTestLevels/ball_player_state.CollectableCount` (+ (`/Game/JasonTestLevels/ball_player_state.CollectableCount` _asball_player_state) 1) _asball_player_state))
    (`KismetSystemLibrary.PrintString` (`KismetStringLibrary.Conv_IntToString` _output_get))
    (`self.K2_DestroyActor`)))

(fn `UserConstructionScript`)