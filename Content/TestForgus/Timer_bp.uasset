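; Level countdown timer actor that ends the level when time runs out.
; On BeginPlay it starts a looping one-second timer that calls DecrementGameTimer to lower TotalTime.
; When TotalTime reaches zero, it shows the EndLevelScreen widget, pauses the game, and switches to UI-only input with a visible mouse cursor.
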(event `self.ReceiveBeginPlay`
  (`KismetSystemLibrary.K2_SetTimer` null "DecrementGameTimer" 1.0 true))

(event `DecrementGameTimer`
  (bind _returnvalue (`GameplayStatics.GetPlayerController` 0))
  (set `self.TotalTime` (- (`self.TotalTime`) 1.0))
  ;[1 1 1] End of Level Condition
  (if (<= (`self.TotalTime`) 0.0)
    (bind _returnvalue_2 (`|CreateWidget` (`self.EndLevelScreen`)))
    (`UserWidget.AddToViewport` _returnvalue_2 0)
    (`GameplayStatics.SetGamePaused` true)
    (`WidgetBlueprintLibrary.SetInputMode_UIOnlyEx` _returnvalue null)
    (set `PlayerController.bShowMouseCursor` true _returnvalue)))

(event `self.ReceiveTick`
  (params (DeltaSeconds :type "Float (single-precision)")))

(fn `UserConstructionScript`)